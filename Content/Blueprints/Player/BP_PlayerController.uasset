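; Player controller that turns Enhanced Input into movement, shooting and jump commands for the possessed character.
; On possess it caches the pawn through a GetCharacterMessage call, and on BeginPlay it adds the IMC_Default mapping context.
; Move, shoot and jump actions forward their start and end phases, plus continuous movement values, to that cached pawn after a validity check.
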(event `self.ReceivePossess`
  (params (PossessedPawn :type "Pawn Object Reference"))
  (bind _characterref (message `/Game/Blueprints/BPI_Character.GetCharacter` PossessedPawn))
  (set `self.CharacterPawn` _characterref))

(event `self.ReceiveBeginPlay`
  (bind _returnvalue (pcsubsystem `EnhancedInputLocalPlayerSubsystem` self))
  (`/Engine/EditorBlueprintResources/StandardMacros.IsValid` _returnvalue
    (:`Is Valid`
      (`EnhancedInputSubsystemInterface.AddMappingContext` _returnvalue "/Game/Blueprints/Input/IMC_Default.IMC_Default" 0 (struct)))))

(event `EnhancedInput|/Game/Blueprints/Input/IA_MoveRight`
  (params (ActionValue :type "Float (double-precision)") (ElapsedSeconds :type "Float (double-precision)") (TriggeredSeconds :type "Float (double-precision)") (InputAction :type "InputAction Object Reference" :default "/Game/Blueprints/Input/IA_MoveRight.IA_MoveRight"))
  (bind _characterpawn (`self.CharacterPawn`))
  (:`Triggered`
    (`/Engine/EditorBlueprintResources/StandardMacros.IsValid` _characterpawn
      (:`Is Valid`
        (`/Game/Blueprints/BP_CharacterBase.Move` _characterpawn ActionValue))))
  (:`Started`
    (`/Engine/EditorBlueprintResources/StandardMacros.IsValid` _characterpawn
      (:`Is Valid`
        (`/Game/Blueprints/BP_CharacterBase.StartMoving` _characterpawn))))
  (:`Completed`
    (`/Engine/EditorBlueprintResources/StandardMacros.IsValid` _characterpawn
      (:`Is Valid`
        (`/Game/Blueprints/BP_CharacterBase.EndMoving` _characterpawn)))))

(event `EnhancedInput|/Game/Blueprints/Input/IA_Shoot`
  (params (ActionValue :type Boolean) (ElapsedSeconds :type "Float (double-precision)") (TriggeredSeconds :type "Float (double-precision)") (InputAction :type "InputAction Object Reference" :default "/Game/Blueprints/Input/IA_Shoot.IA_Shoot"))
  (bind _characterpawn (`self.CharacterPawn`))
  (:`Started`
    (`/Engine/EditorBlueprintResources/StandardMacros.IsValid` _characterpawn
      (:`Is Valid`
        (`/Game/Blueprints/BP_CharacterBase.FireInput` _characterpawn))))
  (:`Completed`
    (`/Engine/EditorBlueprintResources/StandardMacros.IsValid` _characterpawn
      (:`Is Valid`
        (`/Game/Blueprints/BP_CharacterBase.EndFireInput` _characterpawn)))))

(event `EnhancedInput|/Game/Blueprints/Input/IA_Jump`
  (params (ActionValue :type Boolean) (ElapsedSeconds :type "Float (double-precision)") (TriggeredSeconds :type "Float (double-precision)") (InputAction :type "InputAction Object Reference" :default "/Game/Blueprints/Input/IA_Jump.IA_Jump"))
  (bind _characterpawn (`self.CharacterPawn`))
  (bind _characterpawn_2 (`self.CharacterPawn`))
  (:`Started`
    (`/Engine/EditorBlueprintResources/StandardMacros.IsValid` _characterpawn_2
      (:`Is Valid`
        (`/Game/Blueprints/BP_CharacterBase.StartJump` _characterpawn_2))))
  (:`Completed`
    (`/Engine/EditorBlueprintResources/StandardMacros.IsValid` _characterpawn
      (:`Is Valid`
        (`/Game/Blueprints/BP_CharacterBase.EndJump` _characterpawn)))))

(fn `UserConstructionScript`)