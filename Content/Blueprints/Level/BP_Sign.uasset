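; BP_Sign is a level sign that shows text when a character comes near it.
; On BeginPlay it casts its widget component's widget to W_SignUI, caches it and sets its Text.
; Overlaps on the Box trigger show the widget on entry and hide it on exit, only for actors whose GetCharacterMessage call returns a valid result.
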(event `self.ReceiveBeginPlay`
  (bind _asw_sign_ui (cast `/Game/Blueprints/UI/W_SignUI` (`WidgetComponent.GetWidget` (`self.Widget`))))
  (bind _output_get (set `self.SignWidget` _asw_sign_ui))
  (`/Game/Blueprints/UI/W_SignUI.SetText` _output_get (`self.Text`)))

(event `self.Box.OnComponentBeginOverlap`
  (params (OverlappedComponent :type "PrimitiveComponent Object Reference") (OtherActor :type "Actor Object Reference") (OtherComp :type "PrimitiveComponent Object Reference") (OtherBodyIndex :type Integer) (bFromSweep :type Boolean) (SweepResult :type "HitResult Structure (by ref)"))
  (bind _characterref (message `/Game/Blueprints/BPI_Character.GetCharacter` OtherActor))
  (`/Engine/EditorBlueprintResources/StandardMacros.IsValid` _characterref
    (:`Is Valid`
      (`/Game/Blueprints/UI/W_SignUI.Show` (`self.SignWidget`)))))

(event `self.Box.OnComponentEndOverlap`
  (params (OverlappedComponent :type "PrimitiveComponent Object Reference") (OtherActor :type "Actor Object Reference") (OtherComp :type "PrimitiveComponent Object Reference") (OtherBodyIndex :type Integer))
  (bind _characterref (message `/Game/Blueprints/BPI_Character.GetCharacter` OtherActor))
  (`/Engine/EditorBlueprintResources/StandardMacros.IsValid` _characterref
    (:`Is Valid`
      (`/Game/Blueprints/UI/W_SignUI.Hide` (`self.SignWidget`)))))

(fn `UserConstructionScript`)