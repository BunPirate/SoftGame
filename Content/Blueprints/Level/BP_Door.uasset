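; BP_Door is a level door that swaps between open and closed mesh components and opens when the player bumps into it while unlocked.
; Opening shows the open mesh and disables collision on both; closing shows the closed mesh and restores its collision.
; The Open flag sets the initial state at BeginPlay and previews it in the construction script.
; LockDoor and UnlockDoor events toggle the lock.
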(event `self.ReceiveBeginPlay`
  (if (`self.Open?`)
    (`self.OpenDoor`)
    (else
      (`self.CloseDoor`))))

(event `OpenDoor`
  (`SceneComponent.SetVisibility` (`self.DoorOpen`) true false)
  (`SceneComponent.SetVisibility` (`self.DoorClosed`) false false)
  (`PrimitiveComponent.SetCollisionEnabled` (`self.DoorClosed`) "NoCollision")
  (`PrimitiveComponent.SetCollisionEnabled` (`self.DoorOpen`) "NoCollision"))

(event `CloseDoor`
  (`SceneComponent.SetVisibility` (`self.DoorOpen`) false false)
  (`SceneComponent.SetVisibility` (`self.DoorClosed`) true false)
  (`PrimitiveComponent.SetCollisionEnabled` (`self.DoorClosed`) "QueryAndPhysics"))

(event `self.DoorClosed.OnComponentHit`
  (params (HitComponent :type "PrimitiveComponent Object Reference") (OtherActor :type "Actor Object Reference") (OtherComp :type "PrimitiveComponent Object Reference") (NormalImpulse :type "Vector Structure") (Hit :type "HitResult Structure (by ref)"))
  (bind _characterref (message `/Game/Blueprints/BPI_Character.GetCharacter` OtherActor))
  (if (== (`GameplayStatics.GetObjectClass` _characterref) "/Game/Blueprints/Player/BP_PlayerCharacter.BP_PlayerCharacter_C")
    (if (not (`self.Locked?`))
      (`self.OpenDoor`))))

(event `LockDoor`
  (set `self.Locked?` true))

(event `UnlockDoor`
  (set `self.Locked?` false))

(fn `UserConstructionScript`
  (if (`self.Open?`)
    (`SceneComponent.SetVisibility` (`self.DoorOpen`) true false)
    (`SceneComponent.SetVisibility` (`self.DoorClosed`) false false)
    (else
      (`SceneComponent.SetVisibility` (`self.DoorOpen`) false false)
      (`SceneComponent.SetVisibility` (`self.DoorClosed`) true false))))