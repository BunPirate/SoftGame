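; Arena encounter spawner that locks the player between entrance and exit doors until three waves of enemies are cleared.
; The first player overlap with TriggerBox closes and locks both doors, then starts a looping timer.
; The timer prunes invalid enemies and, once none remain, spawns the next wave at random spawnpoint offsets from the actor.
; After the final wave it stops the timer, then unlocks and opens the doors.
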(event `ResetSpawner`
  (set `self.WaveIndex` 0)
  (`KismetArrayLibrary.Array_Clear` (`self.Enemies`)))

(event `TriggerSpawner`
  (bind _entrancedoor (`self.EntranceDoor`))
  (bind _returnvalue (`KismetSystemLibrary.K2_SetTimerDelegate` (delegate `CheckForEnemies`) 0.25 true))
  (`/Game/Blueprints/Level/BP_Door.CloseDoor` _entrancedoor)
  (`/Game/Blueprints/Level/BP_Door.CloseDoor` (`self.ExitDoor`))
  (`/Game/Blueprints/Level/BP_Door.LockDoor` _entrancedoor)
  (`/Game/Blueprints/Level/BP_Door.LockDoor` (`self.ExitDoor`)))

(event `CheckForEnemies`
  (bind _enemies (`self.Enemies`))
  (for (_array_element _array_index) _enemies
    (`/Engine/EditorBlueprintResources/StandardMacros.IsValid` _array_element
      (:`Is Not Valid`
        (`KismetArrayLibrary.Array_Remove` _enemies _array_index))))
  (if (`KismetArrayLibrary.Array_IsEmpty` _enemies)
    (if (> (`self.WaveIndex`) 2)
      (`self.CompleteSpawner`)
      (`KismetSystemLibrary.K2_ClearAndInvalidateTimerHandle` (stale `TriggerSpawner` _returnvalue))
      (else
        (for _array_element_2 (select `int` (`self.WaveIndex`) :`0` (`self.Wave1`) :`1` (`self.Wave2`) :`2` (`self.Wave3`))
          (bind _returnvalue (`|SpawnActorFromClass` _array_element_2 (`KismetMathLibrary.MakeTransform` (+ (`self.K2_GetActorLocation`) (`KismetArrayLibrary.Array_Random` (`self.Spawnpoints`)))) "AdjustIfPossibleButAlwaysSpawn" "OverrideRootScale" null null))
          (`KismetArrayLibrary.Array_AddUnique` (`self.Enemies`) _returnvalue))
        (`/Engine/EditorBlueprintResources/StandardMacros.IncrementInt` (`self.WaveIndex`))))))

(event `CompleteSpawner`
  (bind _entrancedoor (`self.EntranceDoor`))
  (`/Engine/EditorBlueprintResources/StandardMacros.DoOnce` false
    (:`Completed`
      (`/Game/Blueprints/Level/BP_Door.UnlockDoor` _entrancedoor)
      (`/Game/Blueprints/Level/BP_Door.UnlockDoor` (`self.ExitDoor`))
      (`/Game/Blueprints/Level/BP_Door.OpenDoor` _entrancedoor)
      (`/Game/Blueprints/Level/BP_Door.OpenDoor` (`self.ExitDoor`)))))

(event `self.TriggerBox.OnComponentBeginOverlap`
  (params (OverlappedComponent :type "PrimitiveComponent Object Reference") (OtherActor :type "Actor Object Reference") (OtherComp :type "PrimitiveComponent Object Reference") (OtherBodyIndex :type Integer) (bFromSweep :type Boolean) (SweepResult :type "HitResult Structure (by ref)"))
  (bind _characterref (message `/Game/Blueprints/BPI_Character.GetCharacter` OtherActor))
  (if (== (`GameplayStatics.GetObjectClass` _characterref) "/Game/Blueprints/Player/BP_PlayerCharacter.BP_PlayerCharacter_C")
    (`/Engine/EditorBlueprintResources/StandardMacros.DoOnce` false
      (:`Completed`
        (`self.TriggerSpawner`)))))

(fn `UserConstructionScript`)