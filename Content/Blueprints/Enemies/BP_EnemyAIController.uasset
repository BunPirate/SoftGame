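; AI controller for a side-scrolling enemy that patrols left and right, jumps at walls and fires at the player.
; A 0.1-second timer targets players overlapping the pawn's sight radius and sphere-traces ahead for walls, triggering delayed jumps.
; Tick moves the pawn while no player is in range; other timers fire and flip patrol direction.
; The re-randomized walk delay never resets its timer, and a line-of-sight trace is unconnected.
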(event `ShootTimer`
  (bind _character_ref (`self.Character Ref`))
  (if (`self.PlayerInRange`)
    (`/Engine/EditorBlueprintResources/StandardMacros.IsValid` _character_ref
      (:`Is Valid`
        (`/Game/Blueprints/BP_CharacterBase.FireInput` _character_ref)))))

(event `self.ReceivePossess`
  (params (PossessedPawn :type "Pawn Object Reference"))
  (bind _characterref (message `/Game/Blueprints/BPI_Character.GetCharacter` PossessedPawn))
  (set `self.Character Ref` _characterref))

(event `self.ReceiveBeginPlay`
  (`KismetSystemLibrary.K2_SetTimerDelegate` (delegate `AITick`) 0.1 true)
  (`KismetSystemLibrary.K2_SetTimerDelegate` (delegate `SwapPatrolDirection`) (`self.RandomWalkDelay`) true)
  (`KismetSystemLibrary.K2_SetTimerDelegate` (delegate `ShootTimer`) 1.0 true)
  (if (`KismetMathLibrary.RandomBoolWithWeight` 0.5)
    (set `self.PatrolState` "NewEnumerator2")
    (else
      (set `self.PatrolState` "NewEnumerator1"))))

(event `AITick`
  (bind _character_ref (`self.Character Ref`))
  (bind _character_ref_2 (`self.Character Ref`))
  (bind _rootcomponent (`Actor.RootComponent` (`self.Character Ref`)))
  (bind _overlappingactors (`PrimitiveComponent.GetOverlappingActors` (`/Game/Blueprints/BP_CharacterBase.SightRadius` _character_ref_2) "/Game/Blueprints/Player/BP_PlayerCharacter.BP_PlayerCharacter_C"))
  (bind _returnvalue (+ (`SceneComponent.K2_GetComponentLocation` _rootcomponent) (0.0 0.0 100.0)))
  (`/Engine/EditorBlueprintResources/StandardMacros.IsValid` _character_ref_2
    (:`Is Valid`
      (if (`KismetArrayLibrary.Array_IsEmpty` _overlappingactors)
        (set `self.PlayerInRange` false)
        (set `/Game/Blueprints/BP_CharacterBase.Target Actor` null _character_ref)
        (else
          (set `self.PlayerInRange` true)
          (set `/Game/Blueprints/BP_CharacterBase.Target Actor` (`|GetArrayItem` _overlappingactors) _character_ref)))
      ;[1 1 1] Check for wall and jump
      (bind (_outhit _returnvalue_2) (`KismetSystemLibrary.SphereTraceSingleForObjects` :`Start` _returnvalue :`End` (+ _returnvalue (* (`SceneComponent.GetForwardVector` _rootcomponent) (`self.WallCheckRange`))) :`Radius` 100.0 :`ObjectTypes` (`|MakeArray` "ObjectTypeQuery1" :!type "EObjectTypeQuery Enum") :`DrawTime` 0.25))
      (if _returnvalue_2
        (`KismetSystemLibrary.Delay` 1.0)
        (`/Game/Blueprints/BP_CharacterBase.StartJump` (`self.Character Ref`))))))

(event `SwapPatrolDirection`
  (bind _patrolstate (`self.PatrolState`))
  (set `self.RandomWalkDelay` (`KismetMathLibrary.RandomFloatInRange` 1.0 (`self.MaxWalkSeconds`)))
  (if (`|EnumEquality` _patrolstate "NewEnumerator1")
    (set `self.PatrolState` "NewEnumerator2")
    (elif (`|EnumEquality` _patrolstate "NewEnumerator2")
      (set `self.PatrolState` "NewEnumerator1"))))

(event `self.ReceiveTick`
  (params (DeltaSeconds :type "Float (single-precision)"))
  (`/Engine/EditorBlueprintResources/StandardMacros.IsValid` (`self.Character Ref`)
    (:`Is Valid`
      (if (not (`self.PlayerInRange`))
        (`self.Patrol`)))))

(event `Patrol`
  (`/Game/Blueprints/BP_CharacterBase.Move` (`self.Character Ref`) (select `/Game/Blueprints/Enemies/E_PatrolState` (`self.PatrolState`) :`NewEnumerator1` 1.0 :`NewEnumerator2` -1.0)))

(fn `UserConstructionScript`)