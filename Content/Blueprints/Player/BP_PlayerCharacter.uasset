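; Player character that adds checkpoint save/load, a health HUD, weapon aiming and a scrolling parallax background driven by horizontal velocity.
; BeginPlay wipes the single save slot and writes a fresh checkpoint; death reloads it asynchronously.
; Checkpoints store transform, apples, level and "Saved"-tagged actors in a class-keyed map, keeping one transform per class.
; Loading destroys "Saved" and "NotSaved" actors, respawns the map entries and refills health.
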(event Custom|SaveAtCheckpoint
  (bind _returnvalue (SaveGame|DoesSaveGameExist "save1"))
  (if _returnvalue
    (bind _savegame (|AsyncLoadGamefromSlot "save1")
      (:Completed
        (bind _asbp_savegame (Utilities|Casting|CastToBP_Savegame _savegame))
        (CallFunction|SetData _asbp_savegame)
        (|AsyncSaveGametoSlot _asbp_savegame "save1")))
    (else
      (bind _returnvalue_2 (SaveGame|CreateSaveGameObject "/Game/Blueprints/Player/BP_Savegame.BP_Savegame_C"))
      (CallFunction|SetData _returnvalue_2)
      (|AsyncSaveGametoSlot _returnvalue_2 "save1"))))

(event Custom|GetData
  (params (SaveObjectRef :type BP%20Savegame%20Object%20Reference))
  (bind _aliveenemies (Variables|/Game/Blueprints/Player/BP_Savegame.BP_Savegame_C|GetAliveEnemies SaveObjectRef))
  (Utilities|FlowControl|Sequence
    (:then_0
      (Transformation|SetActorTransform (Variables|/Game/Blueprints/Player/BP_Savegame.BP_Savegame_C|GetPlayerPosition SaveObjectRef) false true))
    (:then_1
      (bind _outactors (Actor|GetAllActorsOfClasswithTag "/Script/Engine.Actor" "Saved"))
      (for _array_element _outactors
        (Actor|DestroyActor _array_element)))
    (:then_2
      (bind _outactors_2 (Actor|GetAllActorsOfClasswithTag "/Script/Engine.Actor" "NotSaved"))
      (for _array_element_2 _outactors_2
        (Actor|DestroyActor _array_element_2)))
    (:then_3
      (bind _keys (Utilities|Map|Keys _aliveenemies))
      (bind _values (Utilities|Map|Values _aliveenemies))
      (for (_array_element_3 _array_index) _keys
        (Game|SpawnActorfromClass _array_element_3 (Utilities|Array|Get(acopy) _values _array_index) "AdjustIfPossibleButAlwaysSpawn" 0 0)))
    (:then_4
      (Variables|Default|SetApplesInWorld (Variables|/Game/Blueprints/Player/BP_Savegame.BP_Savegame_C|GetPlayerApples SaveObjectRef)))
    (:then_5
      (Variables|Default|SetHealth (Variables|Default|GetMaxHealth)))))

(event Custom|LoadAtLastCheckpoint
  (bind _savegame (|AsyncLoadGamefromSlot "save1")
    (:Completed
      (bind _asbp_savegame (Utilities|Casting|CastToBP_Savegame _savegame))
      (CallFunction|GetData _asbp_savegame))))

(event Custom|SetData
  (params (SaveObjectRef :type BP%20Savegame%20Object%20Reference))
  (bind _aliveenemies (Variables|/Game/Blueprints/Player/BP_Savegame.BP_Savegame_C|GetAliveEnemies SaveObjectRef))
  (Utilities|FlowControl|Sequence
    (:then_0
      (Variables|/Game/Blueprints/Player/BP_Savegame.BP_Savegame_C|SetPlayerPosition SaveObjectRef (Transformation|GetActorTransform)))
    (:then_1
      (Variables|/Game/Blueprints/Player/BP_Savegame.BP_Savegame_C|SetPlayerApples SaveObjectRef (Variables|Default|GetApplesInWorld)))
    (:then_2
      (Utilities|Map|Clear _aliveenemies)
      (bind _outactors (Actor|GetAllActorsOfClasswithTag "/Script/Engine.Actor" "Saved"))
      (for _array_element _outactors
        (Utilities|Map|Add _aliveenemies (Utilities|GetClass _array_element) (Transformation|GetActorTransform _array_element))))
    (:then_3
      (bind _returnvalue (Game|GetCurrentLevelName true))
      (Variables|/Game/Blueprints/Player/BP_Savegame.BP_Savegame_C|SetLevel SaveObjectRef _returnvalue)
      (Variables|Default|SetHealth (Variables|Default|GetMaxHealth)))))

(event EventBeginPlay
  (|CallParentFunction)
  (bind _returnvalue (Rendering|Material|CreateDynamicMaterialInstance "/Game/Materials/M_ParallaxSprite.M_ParallaxSprite" "None" "None" :!class /Script/Engine.KismetMaterialLibrary))
  (bind _output_get (Variables|Default|SetBackgroundMat _returnvalue))
  (Rendering|Material|SetMaterial (Variables|Default|GetPlane) 0 _output_get)
  (SaveGame|DeleteGameinSlot "save1")
  (CallFunction|SaveatCheckpoint)
  (bind _returnvalue_2 (UserInterface|CreateWidget "/Game/Blueprints/UI/W_Hud.W_Hud_C"))
  (UserInterface|Viewport|AddtoViewport _returnvalue_2 0)
  (Default|InitHealthbar _returnvalue_2 self))

(event EventDie
  (CallFunction|LoadatLastCheckpoint))

(event EventTick
  (params (DeltaSeconds :type Float%20%28single-precision%29))
  (|CallParentFunction DeltaSeconds)
  (CallFunction|PlayerAimWeapon)
  (Variables|Parallax|SetParallaxOffset (+ (Variables|Parallax|GetParallaxOffset) (* (Utilities|Time|GetWorldDeltaSeconds) (Math|Float|MapRangeClamped (.x (Transformation|GetVelocity)) -1e+03 1e+03 -1.0 1.0) 0.01)))
  (if (> (Variables|Parallax|GetParallaxOffset) 1.0)
    (Variables|Parallax|SetParallaxOffset (.Remainder (Math|Float|Division(WholeandRemainder) (Variables|Parallax|GetParallaxOffset) 1.0))))
  (Rendering|Material|SetScalarParameterValue (Variables|Default|GetBackgroundMat) "Offset" (Variables|Parallax|GetParallaxOffset) :!class /Script/Engine.MaterialInstanceDynamic))

(event Input|KeyboardEvents|DebugKey2
  (params (Key :type Key%20Structure :default "None") (ActionValue :type Input%20Action%20Value%20Structure))
  (:Pressed
    (CallFunction|LoadatLastCheckpoint)))

(event Input|KeyboardEvents|DebugKey1
  (params (Key :type Key%20Structure :default "None") (ActionValue :type Input%20Action%20Value%20Structure))
  (:Pressed
    (CallFunction|SaveatCheckpoint)))

(fn ConstructionScript
  (|CallParentFunction))