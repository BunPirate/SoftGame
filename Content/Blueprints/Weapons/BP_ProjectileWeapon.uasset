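; Projectile weapon that fires a burst of confetti projectiles from its FirePoint.
; Shoot runs the parent weapon's logic, then spawns one BP_ConfettiProjectile per pellet at the fire point's transform.
; Each pellet's sphere gets a velocity-change impulse scaled by projectile speed, randomized within a spread cone around the fire point's forward vector.
; The impulse's Y component is zeroed, so launches stay in the world XZ plane.
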(event `self.Shoot`
  (bind _firepoint (`self.FirePoint`))
  (bind (_returnvalue_location _returnvalue_rotation) (`KismetMathLibrary.BreakTransform` (`SceneComponent.K2_GetComponentToWorld` _firepoint)))
  (`parent.Shoot`)
  (for _ (range (`self.NumPellets`))
    (bind _returnvalue (`|SpawnActorFromClass` "/Game/Blueprints/Weapons/Projectiles/BP_ConfettiProjectile.BP_ConfettiProjectile_C" (`KismetMathLibrary.MakeTransform` _returnvalue_location _returnvalue_rotation) "AlwaysSpawn" "OverrideRootScale" null null))
    (`/Engine/EditorBlueprintResources/StandardMacros.IsValid` _returnvalue
      (:`Is Valid`
        (`PrimitiveComponent.AddImpulse` (`/Game/Blueprints/Weapons/Projectiles/BP_ProjectileBase.Sphere` _returnvalue) (`KismetMathLibrary.MakeVector` (.x (* (`KismetMathLibrary.RandomUnitVectorInConeInDegrees` (`SceneComponent.GetForwardVector` _firepoint) (`self.SpreadDegreesHalf`)) (`self.ProjectileSpeed`))) 0.0 (.z (* (`KismetMathLibrary.RandomUnitVectorInConeInDegrees` (`SceneComponent.GetForwardVector` _firepoint) (`self.SpreadDegreesHalf`)) (`self.ProjectileSpeed`)))) "None" true)))))

(fn `UserConstructionScript`
  (`parent.UserConstructionScript`))