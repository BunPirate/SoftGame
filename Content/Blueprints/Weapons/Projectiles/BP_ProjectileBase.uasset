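; Base projectile actor that damages and knocks back what it hits, then destroys itself, with movement kept to the XZ plane.
; Tick resets Y to zero each frame, and a five-second timer destroys projectiles that are still alive.
; On hit, it sends damage through a message call and launches any returned character against the hit normal, scaled by Knockback with Y zeroed.
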(event `self.ReceiveBeginPlay`
  (`KismetSystemLibrary.K2_SetTimerDelegate` (delegate `Die`) 5.0))

(event `Die`
  (`self.K2_DestroyActor`))

(event `self.ReceiveTick`
  (params (DeltaSeconds :type "Float (single-precision)"))
  (bind (_returnvalue_x _returnvalue_y _returnvalue_z) (`KismetMathLibrary.BreakVector` (`self.K2_GetActorLocation`)))
  (`self.K2_SetActorLocation` (`KismetMathLibrary.MakeVector` _returnvalue_x 0.0 _returnvalue_z)))

(event `self.ReceiveHit`
  (params (MyComp :type "PrimitiveComponent Object Reference") (Other :type "Actor Object Reference") (OtherComp :type "PrimitiveComponent Object Reference") (bSelfMoved :type Boolean) (HitLocation :type "Vector Structure") (HitNormal :type "Vector Structure") (NormalImpulse :type "Vector Structure") (Hit :type "HitResult Structure (by ref)"))
  (message `/Game/Blueprints/BPI_Damage.DoDamage` Other (`self.Damage`))
  (bind _characterref (message `/Game/Blueprints/BPI_Character.GetCharacter` Other))
  (`/Engine/EditorBlueprintResources/StandardMacros.IsValid` _characterref
    (:`Is Valid`
      (`Character.LaunchCharacter` _characterref (* (`KismetMathLibrary.MakeVector` (.x HitNormal) 0.0 (.z HitNormal)) (`self.Knockback`) -1.0) false false))
    (:`Is Not Valid`
      _))
  (`self.Die`))

(fn `UserConstructionScript`)