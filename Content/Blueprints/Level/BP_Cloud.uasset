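; BP_Cloud is a cloud actor that drifts through the level as a 2D Paper2D sprite.
; On BeginPlay it picks a random sprite from the CloudSprites array and rolls a random drift speed.
; Each Tick it moves along world X at that speed, scaled by delta time, with no wrapping or despawn logic.
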(event `self.ReceiveBeginPlay`
  (`PaperSpriteComponent.SetSprite` (`self.PaperSprite`) (`KismetArrayLibrary.Array_Random` (`self.CloudSprites`)))
  (set `self.Speed` (`KismetMathLibrary.RandomFloatInRange` 100.0 200.0)))

(event `self.ReceiveTick`
  (params (DeltaSeconds :type "Float (single-precision)"))
  (`self.K2_AddActorWorldOffset` (`KismetMathLibrary.MakeVector` (* DeltaSeconds (`self.Speed`)))))

(fn `UserConstructionScript`)