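; BP_ToffeeApple is a physics-driven toffee apple that sticks to whatever it hits, other than its instigator.
; On impact it stops simulating, enables its box and sphere collision, attaches to the hit component and plays a one-time impact sound.
; Sphere collision starts physics-only and gains queries after a short delay.
; Damage drains its health, and at zero it asks the instigator's character to remove it from the world.
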(event `self.ReceiveBeginPlay`
  (`PrimitiveComponent.SetCollisionEnabled` (`self.Box`) "NoCollision")
  (`PrimitiveComponent.SetCollisionEnabled` (`self.Sphere`) "PhysicsOnly")
  (`KismetSystemLibrary.Delay` 0.5)
  (`PrimitiveComponent.SetCollisionEnabled` (`self.Sphere`) "QueryAndPhysics"))

(event `Freeze`
  (bind _sphere (`self.Sphere`))
  (`PrimitiveComponent.SetSimulatePhysics` _sphere false :!label _label)
  (`PrimitiveComponent.SetCollisionEnabled` _sphere "QueryAndPhysics")
  (`PrimitiveComponent.SetCollisionEnabled` (`self.Box`) "QueryAndPhysics")
  (`self.K2_AttachToComponent` (stale `self.Sphere.OnComponentHit` OtherComp) "None" "KeepWorld" "KeepWorld" "KeepWorld")
  (`/Engine/EditorBlueprintResources/StandardMacros.DoOnce` false
    (:`Completed`
      (`GameplayStatics.PlaySoundAtLocation` "/Game/SFX/Weapons/AppleImpact.AppleImpact" (`self.K2_GetActorLocation`) (struct) 1.0 1.0 0.0 "/Game/SFX/NewSoundAttenuation.NewSoundAttenuation" "/Game/SFX/NewSoundConcurrency.NewSoundConcurrency" null null))))

(event `self.Sphere.OnComponentHit`
  (params (HitComponent :type "PrimitiveComponent Object Reference") (OtherActor :type "Actor Object Reference") (OtherComp :type "PrimitiveComponent Object Reference") (NormalImpulse :type "Vector Structure") (Hit :type "HitResult Structure (by ref)"))
  (if (not (== OtherActor (`self.GetInstigator`)))
    (goto _label)))

(event `/Game/Blueprints/BPI_Damage.DoDamage`
  (params (Damage :type Integer))
  (bind _output_get (set `self.Health` (- (`self.Health`) Damage)))
  (if (<= _output_get 0)
    (bind _characterref (message `/Game/Blueprints/BPI_Character.GetCharacter` (`self.GetInstigator`)))
    (`/Game/Blueprints/BP_CharacterBase.RemoveAppleFromWorld` _characterref self)))

(fn `UserConstructionScript`)