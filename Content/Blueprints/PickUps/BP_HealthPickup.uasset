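; Health pickup actor that restores a fixed amount of the player's health, capped at maximum, on overlap.
; A Timeline started on BeginPlay bobs the apple sprite up and down.
; Box overlap fetches the character via a message call, checks for BP_PlayerCharacter, heals, spawns a Niagara effect, then plays a sound and destroys itself behind a DoOnce.
; RunSlowTime, a timer-driven slow-time event, is marked unused.
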(event `RunSlowTime`
  ;[1 0 0] not being used
  (bind _returnvalue (`KismetSystemLibrary.K2_SetTimer` null "StartSlowingTime" 0.01 true))
  (set `self.TimerHandle` _returnvalue)
  (`KismetSystemLibrary.Delay` 4.5)
  (`KismetSystemLibrary.K2_PauseTimerHandle` (`self.TimerHandle`)))

(event `self.ReceiveBeginPlay`
  (bind (_direction _newtrack_0) (`Timeline|Timeline`)
    (:`Update`
      (`SceneComponent.K2_SetRelativeLocation` (`self.ApplepickupSprite`) (`KismetMathLibrary.VLerp` (0.0 0.0 0.0) (0.0 0.0 15.0) _newtrack_0) false false))))

(event `self.Box.OnComponentBeginOverlap`
  (params (OverlappedComponent :type "PrimitiveComponent Object Reference") (OtherActor :type "Actor Object Reference") (OtherComp :type "PrimitiveComponent Object Reference") (OtherBodyIndex :type Integer) (bFromSweep :type Boolean) (SweepResult :type "HitResult Structure (by ref)"))
  (bind _characterref (message `/Game/Blueprints/BPI_Character.GetCharacter` OtherActor))
  (`/Engine/EditorBlueprintResources/StandardMacros.IsValid` _characterref
    (:`Is Valid`
      (if (== (`GameplayStatics.GetObjectClass` _characterref) "/Game/Blueprints/Player/BP_PlayerCharacter.BP_PlayerCharacter_C")
        (set `/Game/Blueprints/BP_CharacterBase.Health` (`KismetMathLibrary.Clamp` (+ (`/Game/Blueprints/BP_CharacterBase.Health` _characterref) 50) 0 (`/Game/Blueprints/BP_CharacterBase.MaxHealth` _characterref)) _characterref)
        (`NiagaraFunctionLibrary.SpawnSystemAtLocation` "/Game/Particles/NS_Jump.NS_Jump" (`self.K2_GetActorLocation`))
        (`/Engine/EditorBlueprintResources/StandardMacros.DoOnce` false
          (:`Completed`
            (`GameplayStatics.PlaySoundAtLocation` "/Game/SFX/Pickups/CandyCollected.CandyCollected" (`self.K2_GetActorLocation`) (struct) 0.5 1.0 0.0 "/Game/SFX/NewSoundAttenuation.NewSoundAttenuation" "/Game/SFX/NewSoundConcurrency.NewSoundConcurrency" null null)
            (`self.K2_DestroyActor`)))))))

(fn `UserConstructionScript`)