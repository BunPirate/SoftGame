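; Sugar Rush candy pickup that triggers a temporary slow-motion flight effect when the player overlaps its box.
; Collection sounds play, and a HasOverlapped flag limits the effect to one use.
; StartSlowingTime slows both global and character time dilation and sets the player flying with altered movement physics, then restores walking and normal time after a delay.
; The timer-based RunSlowTime path and debug prints are unused.
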(event `RunSlowTime`
  ;[1 0 0] not being used
  (bind _returnvalue (`KismetSystemLibrary.K2_SetTimer` null "StartSlowingTime" 0.01 true))
  (set `self.TimerHandle` _returnvalue)
  (`KismetSystemLibrary.Delay` 4.5)
  (`KismetSystemLibrary.K2_PauseTimerHandle` (`self.TimerHandle`)))

(event `self.Box.OnComponentBeginOverlap`
  (params (OverlappedComponent :type "PrimitiveComponent Object Reference") (OtherActor :type "Actor Object Reference") (OtherComp :type "PrimitiveComponent Object Reference") (OtherBodyIndex :type Integer) (bFromSweep :type Boolean) (SweepResult :type "HitResult Structure (by ref)"))
  (bind _characterref (message `/Game/Blueprints/BPI_Character.GetCharacter` OtherActor))
  (`/Engine/EditorBlueprintResources/StandardMacros.IsValid` _characterref
    (:`Is Valid`
      (`GameplayStatics.PlaySoundAtLocation` "/Game/SFX/Pickups/CandyCollected.CandyCollected" (`self.K2_GetActorLocation`) (struct) 0.5 1.0 0.0 "/Game/SFX/NewSoundAttenuation.NewSoundAttenuation" "/Game/SFX/NewSoundConcurrency.NewSoundConcurrency" null null)
      (if (== (`GameplayStatics.GetObjectClass` _characterref) "/Game/Blueprints/Player/BP_PlayerCharacter.BP_PlayerCharacter_C")
        (if (not (`self.HasOverlapped?`))
          (set `self.HasOverlapped?` true)
          (`self.StartSlowingTime`))))))

(event `StartSlowingTime`
  (set `self.SlowMotion?` true)
  (`GameplayStatics.PlaySound2D` "/Game/SFX/Effects/TimeSlowEffect.TimeSlowEffect" 1.0 1.0 0.0 null null false)
  (bind _characterref (message `/Game/Blueprints/BPI_Character.GetCharacter` (stale `self.Box.OnComponentBeginOverlap` _characterref)))
  (if (`self.SlowMotion?`)
    (`/Engine/EditorBlueprintResources/StandardMacros.DoOnce` false :!label _label
      (:`Completed`
        (bind _output_get (set `Actor.CustomTimeDilation` 0.4 _characterref))
        (bind _charactermovement (`Character.CharacterMovement` _characterref))
        (`CharacterMovementComponent.SetMovementMode` _charactermovement "MOVE_Flying" 0)
        (set `CharacterMovementComponent.Mass` 1.0 _charactermovement)
        (set `CharacterMovementComponent.FallingLateralFriction` 100.0 _charactermovement)
        (set `MovementComponent.Velocity` (`self.TempVelocity`) _charactermovement)
        (bind _output_get_2 (set `CharacterMovementComponent.GravityScale` 1.0 _charactermovement))
        (`GameplayStatics.SetGlobalTimeDilation` _output_get)
        (`KismetSystemLibrary.Delay` 5.0)
        (set `self.Gravity Scale` 1.0)
        (set `CharacterMovementComponent.Mass` 100.0 _charactermovement)
        (`CharacterMovementComponent.SetMovementMode` _charactermovement "MOVE_Walking" 0)
        (set `CharacterMovementComponent.FallingLateralFriction` 0.0 _charactermovement)
        (set `Actor.CustomTimeDilation` 1.0 _characterref)
        (`GameplayStatics.SetGlobalTimeDilation` 1.0)
        (`KismetSystemLibrary.Delay` 1.0)
        (set `self.SlowMotion?` false)
        (set `self.HasOverlapped?` true)
        (goto _label :!via `Reset`)))))

(fn `UserConstructionScript`)