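; One-way 2D platform that lets characters pass through by switching off its collision box.
; A character overlapping the trigger below the platform, or an Interact call, disables PlatformCollision.
; When the character leaves the trigger, collision returns to query-and-physics after a short delay.
; The construction script lays out paper sprite tiles from NumberOfTiles and sizes and offsets both boxes to span the row.
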(event `/Game/Blueprints/Level/BPI_Platform.Interact`
  (`PrimitiveComponent.SetCollisionEnabled` (`self.PlatformCollision`) "NoCollision" :!label _label))

(event `self.PlatformTrigger.OnComponentBeginOverlap`
  (params (OverlappedComponent :type "PrimitiveComponent Object Reference") (OtherActor :type "Actor Object Reference") (OtherComp :type "PrimitiveComponent Object Reference") (OtherBodyIndex :type Integer) (bFromSweep :type Boolean) (SweepResult :type "HitResult Structure (by ref)"))
  (bind _characterref (message `/Game/Blueprints/BPI_Character.GetCharacter` OtherActor))
  (`/Engine/EditorBlueprintResources/StandardMacros.IsValid` _characterref
    (:`Is Valid`
      (goto _label))))

(event `self.PlatformTrigger.OnComponentEndOverlap`
  (params (OverlappedComponent :type "PrimitiveComponent Object Reference") (OtherActor :type "Actor Object Reference") (OtherComp :type "PrimitiveComponent Object Reference") (OtherBodyIndex :type Integer))
  (bind _characterref (message `/Game/Blueprints/BPI_Character.GetCharacter` OtherActor))
  (`/Engine/EditorBlueprintResources/StandardMacros.IsValid` _characterref
    (:`Is Valid`
      (`KismetSystemLibrary.Delay` 0.2)
      (`PrimitiveComponent.SetCollisionEnabled` (`self.PlatformCollision`) "QueryAndPhysics"))))

(fn `UserConstructionScript`
  (bind _platformtrigger (`self.PlatformTrigger`))
  (for _index (range (`self.NumberOfTiles`))
    (`AddComponent|NODE_AddPaperSpriteComponent-0` :`RelativeTransform` (`KismetMathLibrary.MakeTransform` (`KismetMathLibrary.MakeVector` (`KismetMathLibrary.Conv_IntToDouble` (* _index 100)))))
    (`BoxComponent.SetBoxExtent` _platformtrigger (`KismetMathLibrary.MakeVector` (`KismetMathLibrary.Conv_IntToDouble` (* (+ _index 1) 50)) 50.0 15.0) false)
    (`BoxComponent.SetBoxExtent` (`self.PlatformCollision`) (`KismetMathLibrary.MakeVector` (`KismetMathLibrary.Conv_IntToDouble` (* (+ _index 1) 50)) 50.0 15.0) false)
    (bind _returnvalue (`KismetMathLibrary.Conv_IntToDouble` (* _index 50)))
    (`SceneComponent.K2_SetRelativeLocation` _platformtrigger (`KismetMathLibrary.MakeVector` _returnvalue 0.0 -45.0) false false)
    (`SceneComponent.K2_SetRelativeLocation` (`self.PlatformCollision`) (`KismetMathLibrary.MakeVector` _returnvalue 0.0 -15.0) false false)))