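; BP_WeaponBase is a sprite-based weapon that handles firing effects and pickup by the player.
; Semi fire gates shots with a DoOnce and delay, while full auto repeats Shoot on a looping timer until EndFire.
; Shoot spawns particles and sound at FirePoint and plays a recoil timeline whose pitch scales with fire delay, without projectile or damage logic.
; Overlapping its box while unheld makes BP_PlayerCharacter drop its weapon and take this one.
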(event `StartFire`
  (switch `/Game/Blueprints/Weapons/E_Firemode` (`self.Firemode`)
    (:`NewEnumerator0`
      (`/Engine/EditorBlueprintResources/StandardMacros.DoOnce` false :!label _label
        (:`Completed`
          (`self.Shoot`)
          (`KismetSystemLibrary.Delay` (`self.FireDelaySeconds`))
          (goto _label :!via `Reset`))))
    (:`NewEnumerator1`
      (bind _returnvalue (`KismetSystemLibrary.K2_SetTimerDelegate` (delegate `FireAuto`) (`self.FireDelaySeconds`) true))
      (set `self.TimeHandle` _returnvalue)
      (`self.Shoot`))))

(event `EndFire`
  (`KismetSystemLibrary.K2_ClearAndInvalidateTimerHandle` (`self.TimeHandle`)))

(event `Shoot`
  (bind _firepoint (`self.FirePoint`))
  (bind _returnvalue (`SceneComponent.K2_GetComponentLocation` _firepoint))
  (`NiagaraFunctionLibrary.SpawnSystemAtLocation` (`self.ShootParticle`) _returnvalue (`SceneComponent.K2_GetComponentRotation` _firepoint))
  (`GameplayStatics.PlaySoundAtLocation` (`self.FireSound`) _returnvalue (struct) 1.0 1.0 0.0 "/Game/SFX/NewSoundAttenuation.NewSoundAttenuation" "/Game/SFX/NewSoundConcurrency.NewSoundConcurrency" null null)
  (bind (_direction _recoillerp) (`Timeline|Recoil` :!via `PlayFromStart`)
    (:`Update`
      (`SceneComponent.K2_SetRelativeRotation` (`self.WeaponSprite`) (`KismetMathLibrary.RLerp` (struct) (`KismetMathLibrary.MakeRotator` 0.0 (`KismetMathLibrary.FClamp` (* (`self.FireDelaySeconds`) 45.0) 0.0 90.0)) _recoillerp) false false))))

(event `FireAuto`
  (`self.Shoot`))

(event `self.Box.OnComponentBeginOverlap`
  (params (OverlappedComponent :type "PrimitiveComponent Object Reference") (OtherActor :type "Actor Object Reference") (OtherComp :type "PrimitiveComponent Object Reference") (OtherBodyIndex :type Integer) (bFromSweep :type Boolean) (SweepResult :type "HitResult Structure (by ref)"))
  (if (not (`self.Held?`))
    (bind _characterref (message `/Game/Blueprints/BPI_Character.GetCharacter` OtherActor))
    (if (== (`GameplayStatics.GetObjectClass` _characterref) "/Game/Blueprints/Player/BP_PlayerCharacter.BP_PlayerCharacter_C")
      (`/Game/Blueprints/BP_CharacterBase.DropWeapon` _characterref)
      (`/Game/Blueprints/BP_CharacterBase.PickUpWeapon` _characterref self))))

(fn `GetWeapon`
  (returns (NewParam :type "/Game/Blueprints/Weapons/BP_WeaponBase Object Reference"))
  (return self))

(fn `UserConstructionScript`)