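; BP_CrackedPlatform is a platform that cracks while a character overlaps it, breaks, and respawns after a delay.
; Trigger overlap plays the crack flipbook once; leaving stops and rewinds it.
; When the flipbook finishes, the platform hides, disables collision and spawns a Niagara break effect, then a timer restores it with a timeline-driven scale animation.
; Construction randomizes the brick's rotation in quarter turns and applies the play rate.
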(event `self.ReceiveBeginPlay`
  (bind _fb_crackedbrick (`self.FB_CrackedBrick`))
  (`PaperFlipbookComponent.Stop` _fb_crackedbrick)
  (`PaperFlipbookComponent.SetNewTime` _fb_crackedbrick 0.0)
  (`PaperFlipbookComponent.SetLooping` _fb_crackedbrick false))

(event `self.Box1.OnComponentBeginOverlap`
  (params (OverlappedComponent :type "PrimitiveComponent Object Reference") (OtherActor :type "Actor Object Reference") (OtherComp :type "PrimitiveComponent Object Reference") (OtherBodyIndex :type Integer) (bFromSweep :type Boolean) (SweepResult :type "HitResult Structure (by ref)"))
  (bind _characterref (message `/Game/Blueprints/BPI_Character.GetCharacter` OtherActor))
  (`/Engine/EditorBlueprintResources/StandardMacros.IsValid` _characterref
    (:`Is Valid`
      (`/Engine/EditorBlueprintResources/StandardMacros.DoOnce` false :!label _label
        (:`Completed`
          (`PaperFlipbookComponent.PlayFromStart` (`self.FB_CrackedBrick`)))))))

(event `self.Box1.OnComponentEndOverlap`
  (params (OverlappedComponent :type "PrimitiveComponent Object Reference") (OtherActor :type "Actor Object Reference") (OtherComp :type "PrimitiveComponent Object Reference") (OtherBodyIndex :type Integer))
  (bind _fb_crackedbrick (`self.FB_CrackedBrick`))
  (bind _characterref (message `/Game/Blueprints/BPI_Character.GetCharacter` OtherActor))
  (`/Engine/EditorBlueprintResources/StandardMacros.IsValid` _characterref
    (:`Is Valid`
      (`PaperFlipbookComponent.Stop` _fb_crackedbrick)
      (`PaperFlipbookComponent.SetNewTime` _fb_crackedbrick 0.0)
      (goto _label :!via `Reset`))))

(event `self.FB_CrackedBrick.OnFinishedPlaying`
  (`SceneComponent.SetVisibility` (`self.DefaultSceneRoot`) false true)
  (`PrimitiveComponent.SetCollisionEnabled` (`self.Box`) "NoCollision")
  (`PrimitiveComponent.SetCollisionEnabled` (`self.Box1`) "NoCollision")
  (`KismetSystemLibrary.K2_SetTimerDelegate` (delegate `RespawnPlatform`) 6.0)
  (`NiagaraFunctionLibrary.SpawnSystemAtLocation` "/Game/Particles/NS_BlockBreak.NS_BlockBreak" (`self.K2_GetActorLocation`)))

(event `RespawnPlatform`
  (`SceneComponent.SetVisibility` (`self.DefaultSceneRoot`) true true)
  (`PrimitiveComponent.SetCollisionEnabled` (`self.Box`) "QueryAndPhysics")
  (`PrimitiveComponent.SetCollisionEnabled` (`self.Box1`) "QueryOnly")
  (bind (_direction _lerp) (`Timeline|Timeline` :!via `PlayFromStart`)
    (:`Update`
      (`SceneComponent.SetRelativeScale3D` (`self.FB_CrackedBrick`) (`KismetMathLibrary.Conv_DoubleToVector` _lerp)))))

(fn `UserConstructionScript`
  (`SceneComponent.K2_SetRelativeRotation` (`self.FB_CrackedBrick`) (`KismetMathLibrary.MakeRotator` 0.0 (select `int` (`KismetMathLibrary.RandomIntegerInRange` 0 3) :`0` 0.0 :`1` 90.0 :`2` 180.0 :`3` 270.0 :!type "Float (single-precision)")) false false)
  (`PaperFlipbookComponent.SetPlayRate` (`self.FB_CrackedBrick`) (`self.PlayRate`)))