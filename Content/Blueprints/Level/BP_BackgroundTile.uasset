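; BP_BackgroundTile is a sprite background tile that scrolls with parallax and repeats horizontally.
; The construction script applies the configured sprite and offset to Background1.
; Each Tick moves the actor in X and Z by the camera's movement scaled by Parallax, keeping Y fixed.
; When the camera leads by the sprite's X bounds extent or more, it snaps forward using a modulo remainder; only the positive X direction wraps.
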(event `self.ReceiveBeginPlay`
  (set `self.LastCameraPosition` (`PlayerCameraManager.GetCameraLocation` (`GameplayStatics.GetPlayerCameraManager` 0)))
  (set `self.Length` (.x (`.BoxExtent` (`KismetSystemLibrary.GetComponentBounds` (`self.Background1`))))))

(event `self.ReceiveTick`
  (params (DeltaSeconds :type "Float (single-precision)"))
  (bind (_returnvalue_x _returnvalue_y) (`KismetMathLibrary.BreakVector` (`self.K2_GetActorLocation`)))
  (bind _returnvalue_x_2 (`KismetMathLibrary.BreakVector` (`self.K2_GetActorLocation`)))
  (bind (_returnvalue_x_3 _returnvalue_y_2 _returnvalue_z) (`KismetMathLibrary.BreakVector` (`self.K2_GetActorLocation`)))
  (bind _lastcameraposition_x (`KismetMathLibrary.BreakVector` (`self.LastCameraPosition`)))
  (bind _returnvalue_x_4 (`KismetMathLibrary.BreakVector` (`PlayerCameraManager.GetCameraLocation` (`GameplayStatics.GetPlayerCameraManager` 0))))
  (bind _output_get (set `self.DeltaMovement` (* (- (`PlayerCameraManager.GetCameraLocation` (`GameplayStatics.GetPlayerCameraManager` 0)) (`self.LastCameraPosition`)) (`self.Parallax`))))
  (bind (_returnvalue_x_5 _returnvalue_y_3 _returnvalue_z_2) (`KismetMathLibrary.BreakVector` (+ (`self.K2_GetActorLocation`) _output_get)))
  (`self.K2_SetActorLocation` (`KismetMathLibrary.MakeVector` _returnvalue_x_5 _returnvalue_y _returnvalue_z_2))
  (set `self.LastCameraPosition` (`PlayerCameraManager.GetCameraLocation` (`GameplayStatics.GetPlayerCameraManager` 0)))
  (if (>= (- _lastcameraposition_x _returnvalue_x_2) (`self.Length`))
    (`self.K2_SetActorLocation` (`KismetMathLibrary.MakeVector` (+ _returnvalue_x_4 (mod (- _returnvalue_x_4 _returnvalue_x_3) (`self.Length`))) _returnvalue_y_2 _returnvalue_z))))

(fn `UserConstructionScript`
  (`PaperSpriteComponent.SetSprite` (`self.Background1`) (`self.Sprite`))
  (`SceneComponent.K2_SetRelativeLocation` (`self.Background1`) (`self.Offset`) false false))